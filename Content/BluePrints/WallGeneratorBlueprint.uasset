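; A generator blueprint that activates when an ElectricShockBlueprint actor overlaps its box, consuming that actor and toggling the visibility of three linked disappearing walls.
; A dynamic material on the generator mesh turns blue to signify electrification, then reverts to gray after a one-second delay.
; If flagged as a summoner, it then spawns two SlowProjecto actors and one Projecto at three cube transforms cached on BeginPlay, only once.
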(event OnComponentBeginOverlap(Box)
  (params (OverlappedComponent :type Primitive%20Component%20Object%20Reference) (OtherActor :type Actor%20Object%20Reference) (OtherComp :type Primitive%20Component%20Object%20Reference) (OtherBodyIndex :type Integer) (bFromSweep :type Boolean) (SweepResult :type Hit%20Result%20Structure%20%28by%20ref%29))
  ;[1 1 1] Triggering generator activation by key item contact
  (bind _aselectric_shock_blueprint (Utilities|Casting|CastToElectricShockBlueprint OtherActor))
  (Rendering|Material|SetVectorParameterValue (stale EventBeginPlay _returnvalue) "Metal" "(R=0.019700,G=0.340000,B=1.000000,A=1.000000)" :!class /Script/Engine.MaterialInstanceDynamic)
  (Actor|DestroyActor _aselectric_shock_blueprint)
  (Utilities|FlowControl|Sequence
    (:then_0
      (bind _asdisappearing_wall_blueprint (Utilities|Casting|CastToDisappearingWallBlueprint (Variables|Default|GetWall1)))
      (Default|SwitchInvisibilty _asdisappearing_wall_blueprint))
    (:then_1
      (bind _asdisappearing_wall_blueprint_2 (Utilities|Casting|CastToDisappearingWallBlueprint (Variables|Default|GetWall2)))
      (Default|SwitchInvisibilty _asdisappearing_wall_blueprint_2))
    (:then_2
      (bind _asdisappearing_wall_blueprint_3 (Utilities|Casting|CastToDisappearingWallBlueprint (Variables|Default|GetWall3)))
      (Default|SwitchInvisibilty _asdisappearing_wall_blueprint_3))
    (:then_3
      (Utilities|FlowControl|Delay 1.0)
      (Rendering|Material|SetVectorParameterValue (stale EventBeginPlay _returnvalue) "Metal" "(R=0.231000,G=0.231000,B=0.231000,A=1.000000)" :!class /Script/Engine.MaterialInstanceDynamic)
      (if (Variables|Default|GetIsSummoner?)
        (if (not (Variables|Default|GetHasSummoned?))
          (Game|SpawnActorfromClass "/Game/NecessaryFiles/SlowProjecto.SlowProjecto_C" (Variables|Default|GetSpawnLocation) "Undefined" 0 0)
          (Game|SpawnActorfromClass "/Game/NecessaryFiles/SlowProjecto.SlowProjecto_C" (Variables|Default|GetSpawnLocation2) "Undefined" 0 0)
          (Game|SpawnActorfromClass "/Game/ThirdPersonBP/Projecto.Projecto_C" (Variables|Default|GetSpawnLocation3) "Undefined" 0 0)
          (Variables|Default|SetHasSummoned? true))))))

(event EventBeginPlay
  ;[1 1 1] Signify Electrified
  (bind _returnvalue (Rendering|Material|CreateDynamicMaterialInstance (Variables|Default|GetWallGenerator_StaticMesh) 0 "/Game/Meshes/Metal.Metal" "None" :!class /Script/Engine.PrimitiveComponent))
  (Variables|Default|SetSpawnLocation (Transformation|GetWorldTransform (Variables|Default|GetCube)))
  (Variables|Default|SetSpawnLocation2 (Transformation|GetWorldTransform (Variables|Default|GetCube1)))
  (Variables|Default|SetSpawnLocation3 (Transformation|GetWorldTransform (Variables|Default|GetCube2))))

(fn ConstructionScript)