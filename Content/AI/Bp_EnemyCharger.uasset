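; Charger enemy that moves toward the player character when PawnSensing spots it and destroys that character on overlap.
; Bullet overlaps on the capsule briefly change the cube's color through a dynamic material instance created at BeginPlay.
; AnyDamage sets Health to Damage minus Health (operands reversed from a usual subtraction), and Tick destroys the enemy once Health is zero or below.
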(event OnSeePawn(PawnSensing)
  (params (Pawn :type Pawn%20Object%20Reference))
  ;[1 1 1] Tracking Script
  (bind _asnew_character_blueprint (Utilities|Casting|CastToNewCharacterBlueprint Pawn))
  (AI|AIMoveTo self "0, 0, 0" _asnew_character_blueprint 5e+01 false))

(event OnComponentBeginOverlap(CapsuleComponent)
  (params (OverlappedComponent :type Primitive%20Component%20Object%20Reference) (OtherActor :type Actor%20Object%20Reference) (OtherComp :type Primitive%20Component%20Object%20Reference) (OtherBodyIndex :type Integer) (bFromSweep :type Boolean) (SweepResult :type Hit%20Result%20Structure%20%28by%20ref%29))
  ;[1 1 1] Color Change when Damaged
  (Utilities|Casting|CastToNewBulletBlueprint OtherActor)
  (Rendering|Material|SetVectorParameterValue (stale EventBeginPlay _returnvalue) "EnemyC" "(R=1.000000,G=0.009597,B=0.000000,A=1.000000)" :!class /Script/Engine.MaterialInstanceDynamic)
  (Utilities|FlowControl|Delay 0.3)
  (Rendering|Material|SetVectorParameterValue (stale EventBeginPlay _returnvalue) "EnemyC" "(R=1.000000,G=0.906000,B=0.060300,A=1.000000)" :!class /Script/Engine.MaterialInstanceDynamic))

(event EventBeginPlay
  ;[1 1 1] Color Change when Damaged
  (bind _returnvalue (Rendering|Material|CreateDynamicMaterialInstance (Variables|Default|GetCube) 0 "/Game/Meshes/Enemy.Enemy" "None" :!class /Script/Engine.PrimitiveComponent)))

(event Game|Damage|EventAnyDamage
  (params (Damage :type Float%20%28single-precision%29) (DamageType :type Damage%20Type%20Object%20Reference) (InstigatedBy :type Controller%20Object%20Reference) (DamageCauser :type Actor%20Object%20Reference))
  ;[1 1 1] Charger Damage
  (Variables|Default|SetHealth (- Damage (Variables|Default|GetHealth))))

(event EventTick
  (params (DeltaSeconds :type Float%20%28single-precision%29))
  ;[1 1 1] Death script when health is zero
  (if (<= (Variables|Default|GetHealth) 0.0)
    (Actor|DestroyActor)))

(event Collision|EventActorBeginOverlap
  (params (OtherActor :type Actor%20Object%20Reference))
  (bind _asnew_character_blueprint (Utilities|Casting|CastToNewCharacterBlueprint OtherActor))
  (Actor|DestroyActor _asnew_character_blueprint))

(fn ConstructionScript)