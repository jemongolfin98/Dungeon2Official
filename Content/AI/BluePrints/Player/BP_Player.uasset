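; BP_Player is the player character Blueprint, handling jump input, movement and damage.
; Two axis inputs, despite their Look Up/Down and Look Right/Left names, drive movement along the actor's forward and right vectors.
; Any damage reduces Health and swaps the mesh to the Enemyred material for a one-second hit flash before restoring Default, with no death check.
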(event Game|Damage|EventAnyDamage
  (params (Damage :type Float%20%28single-precision%29) (DamageType :type Damage%20Type%20Object%20Reference) (InstigatedBy :type Controller%20Object%20Reference) (DamageCauser :type Actor%20Object%20Reference))
  (Variables|Default|SetHealth (- (Variables|Default|GetHealth) Damage))
  (Rendering|Material|SetMaterial (Variables|Character|GetMesh) 0 "/Game/ThirdPersonBP/enemyred.enemyred")
  (Utilities|FlowControl|Delay 1.0)
  (Rendering|Material|SetMaterial (Variables|Character|GetMesh) 0 "/Game/ThirdPersonBP/Default.Default"))

(event Input|ActionEvents|InputActionJump
  (params (Key :type Key%20Structure))
  (:Pressed
    (Character|Jump)))

(event Input|AxisEvents|InputAxisLookUp/Down
  (params (AxisValue :type Float%20%28single-precision%29))
  (Pawn|Input|AddMovementInput (Transformation|GetActorForwardVector) AxisValue false))

(event Input|AxisEvents|InputAxisLookRight/Left
  (params (AxisValue :type Float%20%28single-precision%29))
  (Pawn|Input|AddMovementInput (Transformation|GetActorRightVector) AxisValue false))

(fn ConstructionScript)