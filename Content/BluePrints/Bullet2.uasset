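; Bullet2 is a projectile actor that damages NewCharacterBlueprint characters it touches and destroys itself after ten seconds.
; A box overlap casts the other actor to that character and subtracts a fixed amount from its CurrentHealth, then destroys the bullet.
; If that health is already at or below zero, the overlap destroys the character instead and leaves the bullet alive.
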(event OnComponentBeginOverlap(Box)
  (params (OverlappedComponent :type Primitive%20Component%20Object%20Reference) (OtherActor :type Actor%20Object%20Reference) (OtherComp :type Primitive%20Component%20Object%20Reference) (OtherBodyIndex :type Integer) (bFromSweep :type Boolean) (SweepResult :type Hit%20Result%20Structure%20%28by%20ref%29))
  ;[1 1 1] Bullet Damage // Death Trigger
  (bind _asnew_character_blueprint (Utilities|Casting|CastToNewCharacterBlueprint OtherActor))
  (if (<= (Variables|/Game/BluePrints/NewCharacterBlueprint.NewCharacterBlueprint_C|GetCurrentHealth _asnew_character_blueprint) 0.0)
    (Actor|DestroyActor _asnew_character_blueprint)
    (else
      (Variables|/Game/BluePrints/NewCharacterBlueprint.NewCharacterBlueprint_C|SetCurrentHealth _asnew_character_blueprint (- (Variables|/Game/BluePrints/NewCharacterBlueprint.NewCharacterBlueprint_C|GetCurrentHealth _asnew_character_blueprint) 0.2))
      (Actor|DestroyActor))))

(event EventBeginPlay
  (Utilities|FlowControl|Delay 1e+01)
  (Actor|DestroyActor))

(fn ConstructionScript)