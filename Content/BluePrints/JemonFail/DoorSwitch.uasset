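; DoorSwitch is a door Blueprint that opens temporarily when its linked Switch reports a hit.
; It binds to the switch's hit event on BeginPlay; if locked, it turns the lock light green, raises the door mesh, waits, then lowers it, turns red and relocks.
; The construction script sets the light colour from IsLocked.
; MoveComponentTo drives the movement, leaving a DoorMove timeline unused.
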(event Custom|UnlockDoor
  (params (Switch :type Generator%20Static%20Mesh%20Blueprint%20Object%20Reference))
  (bind _doorproxmesh (Variables|Default|GetDoorProxMesh))
  (bind _locklight (Variables|Default|GetLocklight))
  ;[1 1 1] Call to generator function, allowing generator activation to trigger door
  (if (== Switch (Variables|Default|GetSwitch))
    ;[1 1 1] Checks if locked or not, activates if locked
    (if (Variables|Default|GetIsLocked)
      (Variables|Default|SetIsLocked false)
      ;[1 1 1] Activates door movement
      (Rendering|Components|Light|SetLightColor _locklight "(R=0.051838,G=0.333333,B=0.020268,A=1.000000)" true)
      (Components|MoveComponentTo _doorproxmesh (Math|Vector|MakeVector 0.0 0.0 3e+02) "0, 0, 0" true true 1.0 false)
      (Utilities|FlowControl|Delay 4.0)
      (Rendering|Components|Light|SetLightColor _locklight "(R=1.000000,G=0.000000,B=0.000000,A=1.000000)" true)
      (Components|MoveComponentTo _doorproxmesh "0, 0, 0" "0, 0, 0" true true 1.0 false)
      (Variables|Default|SetIsLocked true))))

(event EventBeginPlay
  ;[1 1 1] Call to generator function, allowing generator activation to trigger door
  (EventDispatchers|BindEventtoSwitchHit (Variables|Default|GetSwitch) (delegate Custom|UnlockDoor)))

(fn ConstructionScript
  (bind _locklight (Variables|Default|GetLocklight))
  ;[1 1 1] Controls door light notifying red for locked green for unlocked
  (if (Variables|Default|GetIsLocked)
    (Rendering|Components|Light|SetLightColor _locklight "(R=1.000000,G=0.000000,B=0.000000,A=1.000000)" true)
    (else
      (Rendering|Components|Light|SetLightColor _locklight "(R=0.051838,G=0.333333,B=0.020268,A=1.000000)" true))))